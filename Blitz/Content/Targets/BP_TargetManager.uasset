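; Target manager for a timed shooting-range-style minigame that spawns BP_Target actors, keeps score and shows a countdown.
; StartCountdown activates a round for Time seconds, then resets the timer and passes the score to BP_ScoreBoard.
; While active, Tick spawns one target at a random point in the box whenever CanSpawn is set, and uses a looping Delay to count down.
; When idle, it clears both texts and destroys any leftover target.
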(event `SpawnTarget`
  (bind _returnvalue (`|SpawnActorFromClass` "/Game/Targets/BP_Target.BP_Target_C" (`KismetMathLibrary.MakeTransform` (`KismetMathLibrary.RandomPointInBoundingBox` (`SceneComponent.K2_GetComponentLocation` (`self.DefaultSceneRoot`)) (`BoxComponent.BoxExtent` (`self.Box`)))) "Undefined" "MultiplyWithRoot" null null)))

(event `StartCountdown`
  (if (not (`self.IsActive`))
    (set `self.IsActive` true)
    (set `self.CurrentScore` 0)
    (`KismetSystemLibrary.Delay` (`self.Time`))
    (set `self.IsActive` false)
    (set `self.Time` 10.0)
    (bind _returnvalue (`GameplayStatics.GetActorOfClass` "/Game/Targets/BP_ScoreBoard.BP_ScoreBoard_C"))
    (`/Game/Targets/BP_ScoreBoard.CheckScore` _returnvalue (`self.CurrentScore`))))

(event `self.ReceiveTick`
  (params (DeltaSeconds :type "Float (single-precision)"))
  (if (`self.IsActive`) :!label _label
    (`|ExecutionSequence`
      (:`then_0`
        (if (`self.CanSpawn`)
          (`self.SpawnTarget`)
          (set `self.CanSpawn` false)
          (`TextRenderComponent.K2_SetText` (`self.Score`) (`|FormatText` "Score: {Score}" (`self.CurrentScore`)))))
      (:`then_1`
        (`TextRenderComponent.K2_SetText` (`self.TextRender`) (`KismetTextLibrary.Conv_DoubleToText` (`self.Time`) "HalfToEven"))
        (`KismetSystemLibrary.Delay` 1.0)
        (set `self.Time` (- (`self.Time`) 1.0))
        (goto _label)))
    (else
      (`TextRenderComponent.K2_SetText` (`self.TextRender`) "")
      (`TextRenderComponent.K2_SetText` (`self.Score`) "")
      (if (`KismetSystemLibrary.IsValid` (stale `SpawnTarget` _returnvalue))
        (`self.K2_DestroyActor` (stale `SpawnTarget` _returnvalue))
        (set `self.CanSpawn` true)))))

(event `IncreaseScore`
  (params (Score :type Integer))
  (set `self.CurrentScore` (+ (`self.CurrentScore`) Score)))

(fn `UserConstructionScript`)